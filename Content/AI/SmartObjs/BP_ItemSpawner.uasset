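; BP_ItemSpawner is an actor that spawns smart object items at placed target points and sends overlapping AI to use one.
; The construction script sizes the sphere to Radius and adds an arrow for each TargetPoint within it.
; BeginPlay creates a BP_Item child actor per arrow.
; Sphere overlap claims the first available item slot and starts MoveToAndUseSmartObjectWithGameplayInteraction on the actor's AI controller, locking AI logic.
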(event OnComponentBeginOverlap(Sphere)
  (params (OverlappedComponent :type Primitive%20Component%20Object%20Reference) (OtherActor :type Actor%20Object%20Reference) (OtherComp :type Primitive%20Component%20Object%20Reference) (OtherBodyIndex :type Integer) (bFromSweep :type Boolean) (SweepResult :type Hit%20Result%20Structure%20%28by%20ref%29))
  (bind _claimedhandle (CallFunction|FindFreeSmartObject OtherActor))
  (|MovetoandUseSmartObjectwithGameplayInteraction (AI|GetAIController OtherActor) _claimedhandle true
    (:OnSucceeded
      (Development|PrintString "Hello"))))

(event EventBeginPlay
  (for _array_element (Variables|Default|GetArrows)
    (bind _returnvalue (AddComponent|AddChildActorComponent false (Math|Transform|MakeTransform (.location (Transformation|GetWorldTransform _array_element)) (.rotation (Transformation|GetWorldTransform _array_element)) "1.000000,1.000000,1.000000")))
    (ChildActorComponent|SetChildActorClass _returnvalue "/Game/AI/SmartObjs/BP_Item.BP_Item_C")))

(fn ConstructionScript
  (Components|Sphere|SetSphereRadius (Variables|Default|GetSphere) (Variables|settings|GetRadius) true)
  (CallFunction|AddArrowsasSpawnPoints))

(fn AddArrowsasSpawnPoints
  (for _array_element (CallFunction|GetAllActorsOfClassWithinRadius self "/Script/Engine.TargetPoint" (Variables|settings|GetRadius))
    (bind _returnvalue (AddComponent|AddArrowComponent false (Math|Transform|MakeTransform (.location (Transformation|GetActorTransform _array_element)) (.rotation (Transformation|GetActorTransform _array_element)) "1.000000,1.000000,1.000000")))
    (Utilities|Array|AddUnique (Variables|Default|GetArrows) _returnvalue)))

(fn FindFreeSmartObject
  (params (Actor :type Actor%20Object%20Reference))
  (bind _array_element (Utilities|Array|ForEachLoopwithBreak (Actor|GetAllChildActors true) :!label _label)
    (:LoopBody
      (bind _asbp_item (Utilities|Casting|CastToBP_Item _array_element))
      (bind (_outresults _returnvalue) (Class|SmartObjectBlueprintFunctionLibrary|FindSmartObjectsinComponent (Utilities|Struct|MakeSmartObjectRequestFilter "(GameplayTags=)" "Normal") (Variables|/Game/AI/SmartObjs/BP_Item.BP_Item_C|GetSmartObject _asbp_item) Actor))
      (if _returnvalue
        (bind _returnvalue_2 (Class|SmartObjectBlueprintFunctionLibrary|MarkSmartObjectSlotasClaimed (.slothandle (Utilities|Array|Get(acopy) _outresults)) Actor "Normal"))
        (LocalVariables|SetClaimed _returnvalue_2)
        (goto _label Break)))
    (:Completed
      (return (LocalVariables|GetClaimed)))))