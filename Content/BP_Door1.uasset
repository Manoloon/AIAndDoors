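; BP_Door1 is a physics-driven door that can be used through interface calls.
; The IUse event switches the Door component's linear and angular damping, low while In is true and very high otherwise, so it moves freely only during use.
; IGetKnob returns the knob location and the Door component to the caller.
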(event EventBeginPlay)

(event Collision|EventActorBeginOverlap
  (params (OtherActor :type Actor%20Object%20Reference)))

(event EventTick
  (params (DeltaSeconds :type Float%20%28single-precision%29)))

(event EventIUse
  (params (in :type Boolean) (NewParam :type Scene%20Component%20Object%20Reference))
  (bind _door (Variables|Default|Getdoor))
  (bind _door_2 (Variables|Default|Getdoor))
  (if in
    (Class|PrimitiveComponent|SetLinearDamping _door_2 2e+01)
    (Class|PrimitiveComponent|SetAngularDamping _door_2 2e+01)
    (else
      (Class|PrimitiveComponent|SetLinearDamping _door 5e+02)
      (Class|PrimitiveComponent|SetAngularDamping _door 5e+02))))

(fn ConstructionScript)

(fn IGetKnob
  (return (Variables|Default|GetKnobLocation) (Variables|Default|Getdoor)))