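; Lockable non-physics door that a user swings through interface yaw input, clamped to opening limits, with squeak, open and shut sounds.
; Two Enter triggers snap the unlocked, idle door fully open either way for pawns.
; A pawn leaving Box starts a delayed looping timer that interpolates the door back to its initial rotation, pausable by use.
; Lock state drives the outline material and the NavLink's smart link.
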(event OnComponentEndOverlap(Box)
  (params (OverlappedComponent :type Primitive%20Component%20Object%20Reference) (OtherActor :type Actor%20Object%20Reference) (OtherComp :type Primitive%20Component%20Object%20Reference) (OtherBodyIndex :type Integer))
  ;[1 1 1] close auto
  (Utilities|Casting|CastToPawn OtherActor)
  (Variables|Default|SetIn%20use false)
  (Class|AudioComponent|SetPaused (Variables|Default|GetSqueak) false)
  (bind _returnvalue (Utilities|Time|SetTimerbyEvent (delegate Custom|CloseDoor) 0.01 true 2.0))
  (Variables|Default|SetTHClose _returnvalue))

(event OnComponentBeginOverlap(Enter)
  (params (OverlappedComponent :type Primitive%20Component%20Object%20Reference) (OtherActor :type Actor%20Object%20Reference) (OtherComp :type Primitive%20Component%20Object%20Reference) (OtherBodyIndex :type Integer) (bFromSweep :type Boolean) (SweepResult :type Hit%20Result%20Structure%20%28by%20ref%29))
  (if (Variables|Settings|GetIsUnlock)
    (if (not (Variables|Default|GetIn%20use))
      (Utilities|Casting|CastToPawn OtherActor)
      (Utilities|Time|ClearandInvalidateTimerbyHandle (Variables|Default|GetTHClose))
      (Variables|Default|SetIn%20use true)
      (Transformation|SetRelativeRotation (Variables|Default|Getdoor) (Math|Rotator|MakeRotator 0.0 0.0 (Variables|Settings|GetMinOpened)) false false))))

(event OnComponentBeginOverlap(Enter2)
  (params (OverlappedComponent :type Primitive%20Component%20Object%20Reference) (OtherActor :type Actor%20Object%20Reference) (OtherComp :type Primitive%20Component%20Object%20Reference) (OtherBodyIndex :type Integer) (bFromSweep :type Boolean) (SweepResult :type Hit%20Result%20Structure%20%28by%20ref%29))
  (if (Variables|Settings|GetIsUnlock)
    (if (not (Variables|Default|GetIn%20use))
      (Utilities|Casting|CastToPawn OtherActor)
      (Utilities|Time|ClearandInvalidateTimerbyHandle (Variables|Default|GetTHClose))
      (Variables|Default|SetIn%20use true)
      (Transformation|SetRelativeRotation (Variables|Default|Getdoor) (Math|Rotator|MakeRotator 0.0 0.0 (Variables|Settings|GetMaxOpened)) false false))))

(event Custom|CloseDoor
  (bind _door (Variables|Default|Getdoor))
  (bind _relativerotation (Variables|/Script/Engine.SceneComponent|GetRelativeRotation _door))
  ;[1 1 1] close
  (Transformation|SetRelativeRotation (Variables|Default|Getdoor) (Math|Interpolation|RInterpTo _relativerotation (Variables|Default|GetFirstRot) (Utilities|Time|GetWorldDeltaSeconds) 2.0) false false)
  (CallFunction|PlaySqueak)
  (if (Math|Float|NearlyEqual(Float) (.yaw (Variables|Default|GetFirstRot)) (.Yaw (Math|Rotator|BreakRotator _relativerotation)) 1.0)
    (Audio|Components|Audio|Stop (Variables|Default|GetSqueak))
    (Utilities|FlowControl|DoOnce true :!label _label
      (:Completed
        (Audio|SpawnSoundAttached "/Game/audio/Bedroom/Shut/S23_Door_Bedroom_Reverb_Shut_04_Cue.S23_Door_Bedroom_Reverb_Shut_04_Cue" (Variables|Default|Getdoor) "None" "0, 0, 0" "0, 0, 0" "KeepRelativeOffset" false 1.0 1.0 0.0 0 0)
        (Utilities|Time|ClearandInvalidateTimerbyHandle (Variables|Default|GetTHClose))
        (CallFunction|ResetOpenSound)))
    (else
      (goto _label Reset))))

(event Custom|StartOpen
  (Utilities|FlowControl|DoOnce false
    (:Completed
      (bind _returnvalue (Audio|SpawnSoundAttached "/Game/audio/Bedroom/Open/S23_Door_Bedroom_Open_01_Cue.S23_Door_Bedroom_Open_01_Cue" (Variables|Default|Getdoor) "None" "0, 0, 0" "0, 0, 0" "KeepRelativeOffset" false 1.0 1.0 0.0 0 0))
      (Variables|Default|SetStartOpenDoor _returnvalue))))

(event Custom|LockUnlockDoor
  (bind _isa (Utilities|FlowControl|FlipFlop)
    (:A
      _)
    (:B
      _))
  (Variables|Settings|SetIsUnlock _isa)
  (CallFunction|DoorLock))

(event Custom|ResetOpenSound
  (Utilities|FlowControl|DoOnce false) ; enters at Reset
)

(event EventEndPlay
  (params (EndPlayReason :type EEndPlayReason%20Enum :default "Destroyed"))
  (Utilities|Time|ClearandInvalidateTimerbyHandle (Variables|Default|GetTHClose)))

(event EventIUse
  (params (in :type Boolean))
  ;[1 1 1] use
  (bind _output_get (Variables|Default|SetIn%20use in))
  (if _output_get
    (Utilities|Time|PauseTimerbyHandle (Variables|Default|GetTHClose))
    (else
      (Utilities|Time|UnpauseTimerbyHandle (Variables|Default|GetTHClose))
      (Audio|Components|Audio|Stop (Variables|Default|GetSqueak)))))

(event EventBeginPlay)

(event EventIFeedYaw
  (params (Feed :type Float%20%28double-precision%29))
  (bind _returnvalue (* Feed 0.5))
  ;[1 1 1] feed yaw
  (if (Variables|Settings|GetIsUnlock)
    (if (== _returnvalue 0.0)
      (CallFunction|StartOpen))
    (Utilities|FlowControl|Sequence
      (:then_0
        (CallFunction|PlaySqueak))
      (:then_1
        (Variables|Default|SetTargetYaw (Math|Float|Clamp(Float) (.yaw (Math|Rotator|CombineRotators (Variables|/Script/Engine.SceneComponent|GetRelativeRotation (Variables|Default|Getdoor)) (Math|Rotator|MakeRotator 0.0 0.0 _returnvalue))) (Variables|Settings|GetMinOpened) (Variables|Settings|GetMaxOpened)))
        (Transformation|SetRelativeRotation (Variables|Default|Getdoor) (Math|Rotator|MakeRotator 0.0 0.0 (Variables|Default|GetTargetYaw)) false false)
        (Class|AudioComponent|SetPaused (Variables|Default|GetSqueak) (Math|Boolean|ORBoolean (== (Variables|Default|GetTargetYaw) 0.0) (== (Variables|Default|GetTargetYaw) -8e+01) (== Feed 0.0)))))))

(fn ConstructionScript
  (Variables|Default|SetFirstRot (Variables|/Script/Engine.SceneComponent|GetRelativeRotation (Variables|Default|Getdoor)))
  (CallFunction|DoorLock))

(fn PlaySqueak
  (if (not (Audio|Components|Audio|IsPlaying (Variables|Default|GetSqueak)))
    (Audio|Components|Audio|Play (Variables|Default|GetSqueak) 0.0)))

(fn DoorLock
  (bind _isunlock (Variables|Settings|GetIsUnlock))
  (bind _navlink (Variables|Settings|GetNavLink))
  (Rendering|Material|SetMaterial (Variables|Default|Getoutline) 0 (select _isunlock "/Game/M_DoorOpen.M_DoorOpen" "/Game/M_DoorLocked.M_DoorLocked"))
  (Utilities|IsValid _navlink
    (:Is%20Valid
      (Class|NavLinkProxy|SetSmartLinkEnabled _navlink _isunlock))))

(fn IGetKnob
  (return (Variables|Default|GetKnobLocation) (Variables|Default|Getdoor)))